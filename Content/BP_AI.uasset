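; BP_AI is an AI Blueprint that turns perception updates into a "hasSeenPlayer?" Blackboard flag on its AI controller.
; A successful sense cancels the forget timer and sets the flag true, without checking which actor was sensed.
; A failed sense starts a short timer that clears the flag on expiry, giving a grace period before forgetting.
; Debug strings print at each stage.
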(event OnTargetPerceptionUpdated(AIPerception)
  (params (Actor :type Actor%20Object%20Reference) (Stimulus :type AI%20Stimulus%20Structure))
  (Variables|Default|SetPerceivedActor Actor)
  (if (.bSuccessfullySensed (Utilities|Struct|BreakAIStimulus Stimulus))
    (Utilities|Time|ClearandInvalidateTimerbyHandle (Variables|Default|GetTargetLostTimer))
    (Development|PrintString "i see you")
    (AI|Components|Blackboard|SetValueasBool (AI|GetBlackboard (AI|GetAIController self)) (Utilities|Name|MakeLiteralName "hasSeenPlayer?") true)
    (else
      (bind _returnvalue (Utilities|Time|SetTimerbyEvent (delegate Custom|TargetLost) 2.0))
      (Variables|Default|SetTargetLostTimer _returnvalue)
      (Development|PrintString "I lost you"))))

(event Custom|TargetLost
  (Development|PrintString "I forgot you")
  (AI|Components|Blackboard|SetValueasBool (AI|GetBlackboard (AI|GetAIController self)) (Utilities|Name|MakeLiteralName "hasSeenPlayer?") false))

(fn ConstructionScript)