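; BP_RotatingDoor is an interactable locked door that swings open when the player holds the matching key.
; It caches the BP_Player on BeginPlay and checks that player's AcquiredKey enum when Interact fires.
; With the right key, a DoorRotate timeline lerps DoorRoot's relative rotation through 90 degrees and flags the door as opened.
; Otherwise it prints a message that the player lacks the key to this room.
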(event EventBeginPlay
  (bind _asbp_player (Utilities|Casting|CastToBP_Player (Game|GetPlayerCharacter 0)))
  (Variables|Default|SetPlayer _asbp_player))

(event EventInteract
  (if (Utilities|Enum|Equal(Enum) (Variables|/Game/BP_Player.BP_Player_C|GetAcquiredKey (Variables|Default|GetPlayer)) "NewEnumerator1")
    (Development|PrintString "Interacted with RotatingDoor")
    (bind _rotate (Timeline|DoorRotate Play)
      (:Update
        (Transformation|SetRelativeRotation (Variables|Default|GetDoorRoot) (Math|Rotator|Lerp(Rotator) "0, 0, 0" "0.000000,90.000000,0.000000" _rotate) false false)
        (Variables|Default|SetRotatingDoorOpened true)))
    (else
      (Development|PrintString "You don't have the key to this room"))))

(fn ConstructionScript)