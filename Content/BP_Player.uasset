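; Player Blueprint that lets the player interact with keys, rotating doors and sliding doors.
; A sphere overlap casts the nearby actor, stores it and sets an InteractionConditions state, ignoring already-opened doors; ending the overlap clears the state.
; Tick polls that state to show or hide the prompt in the gameplay widget created on BeginPlay.
; Pressing E switches on the state to trigger the stored actor's interaction.
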(event OnComponentBeginOverlap(Sphere)
  (params (OverlappedComponent :type Primitive%20Component%20Object%20Reference) (OtherActor :type Actor%20Object%20Reference) (OtherComp :type Primitive%20Component%20Object%20Reference) (OtherBodyIndex :type Integer) (bFromSweep :type Boolean) (SweepResult :type Hit%20Result%20Structure%20%28by%20ref%29))
  (bind _asbp_key (Utilities|Casting|CastToBP_Key OtherActor)
    (:then
      (Variables|Default|SetOverlapped_Key _asbp_key)
      (Variables|Default|SetInteractionConditions "NewEnumerator0"))
    (:CastFailed
      (bind _asbp_rotating_door (Utilities|Casting|CastToBP_RotatingDoor OtherActor)
        (:then
          (bind _output_get (Variables|Default|SetOverlapped_RotatingDoor _asbp_rotating_door))
          (if (not (Variables|/Game/BP_RotatingDoor.BP_RotatingDoor_C|GetRotatingDoorOpened _output_get))
            (Variables|Default|SetInteractionConditions "NewEnumerator2")))
        (:CastFailed
          (bind _asbp_sliding_door (Utilities|Casting|CastToBP_SlidingDoor OtherActor))
          (bind _output_get_2 (Variables|Default|SetOverlapped_SlidingDoor _asbp_sliding_door))
          (if (not (Variables|/Game/BP_SlidingDoor.BP_SlidingDoor_C|GetSlidingDoorOpened _output_get_2))
            (Variables|Default|SetInteractionConditions "NewEnumerator3")))))))

(event OnComponentEndOverlap(Sphere)
  (params (OverlappedComponent :type Primitive%20Component%20Object%20Reference) (OtherActor :type Actor%20Object%20Reference) (OtherComp :type Primitive%20Component%20Object%20Reference) (OtherBodyIndex :type Integer))
  (bind _asbp_key (Utilities|Casting|CastToBP_Key OtherActor)
    (:then
      (Variables|Default|SetOverlapped_Key _asbp_key)
      (Variables|Default|SetInteractionConditions "NewEnumerator1"))
    (:CastFailed
      (bind _asbp_rotating_door (Utilities|Casting|CastToBP_RotatingDoor OtherActor)
        (:then
          (Variables|Default|SetOverlapped_RotatingDoor _asbp_rotating_door)
          (Variables|Default|SetInteractionConditions "NewEnumerator1"))
        (:CastFailed
          (bind _asbp_sliding_door (Utilities|Casting|CastToBP_SlidingDoor OtherActor))
          (Variables|Default|SetOverlapped_SlidingDoor _asbp_sliding_door)
          (Variables|Default|SetInteractionConditions "NewEnumerator1"))))))

(event EventBeginPlay
  (bind _returnvalue (UserInterface|CreateWidget "/Game/WD_Gameplay.WD_Gameplay_C"))
  (bind _output_get (Variables|Default|SetWD_Gameplay _returnvalue))
  (UserInterface|Viewport|AddtoViewport _output_get 0))

(event EventTick
  (params (DeltaSeconds :type Float%20%28single-precision%29))
  (bind _wd_gameplay (Variables|Default|GetWD_Gameplay))
  (if (Utilities|Enum|NotEqual(Enum) (Variables|Default|GetInteractionConditions) "NewEnumerator1")
    (Default|DisplayInteractionText _wd_gameplay)
    (else
      (Default|UndisplayInteractionText _wd_gameplay))))

(event Input|KeyboardEvents|E
  (params (Key :type Key%20Structure :default "None"))
  (:Pressed
    (switch Utilities|FlowControl|Switch|SwitchonInteractionConditions (Variables|Default|GetInteractionConditions)
      (:NewEnumerator0
        (Default|Interact (Variables|Default|GetOverlapped_Key)))
      (:NewEnumerator2
        (Class|IInteractables|Interact(Message) (Variables|Default|GetOverlapped_RotatingDoor)))
      (:NewEnumerator3
        (Class|IInteractables|Interact(Message) (Variables|Default|GetOverlapped_SlidingDoor))))))

(fn ConstructionScript)