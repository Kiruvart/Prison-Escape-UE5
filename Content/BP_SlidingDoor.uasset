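; BP_SlidingDoor is a key-locked door that opens when the player interacts with it.
; On BeginPlay it caches the player as BP_Player, and on Interact it checks that player's AcquiredKey against one specific enum value.
; With the matching key, a timeline rotates RotatingPoint toward a quarter-turn and sets SlidingDoorOpened; otherwise it prints a wrong-key message.
; Despite its name, the door swings by rotation rather than sliding.
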(event EventBeginPlay
  (bind _asbp_player (Utilities|Casting|CastToBP_Player (Game|GetPlayerCharacter 0)))
  (Variables|Default|SetPlayer _asbp_player))

(event EventInteract
  (if (Utilities|Enum|Equal(Enum) (Variables|/Game/BP_Player.BP_Player_C|GetAcquiredKey (Variables|Default|GetPlayer)) "NewEnumerator3")
    (Development|PrintString "Interacted with SlidingDoor")
    (bind _newtrack_0 (Timeline|DoorRotate Play)
      (:Update
        (Transformation|SetRelativeRotation (Variables|Default|GetRotatingPoint) (Math|Rotator|Lerp(Rotator) "0, 0, 0" "0.000000,-90.000000,0.000000" _newtrack_0) false false)
        (Variables|Default|SetSlidingDoorOpened true)))
    (else
      (Development|PrintString "You don't have the correct key"))))

(fn ConstructionScript)