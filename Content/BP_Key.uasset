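; BP_Key is an interactable key pickup that hands one of three key types to the player.
; On BeginPlay it caches the player character as BP_Player.
; On Interact it switches on KeyIndex, prints which key was acquired, overwrites the player's AcquiredKey enum with the matching value, then destroys itself.
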(event EventBeginPlay
  (bind _asbp_player (Utilities|Casting|CastToBP_Player (Game|GetPlayerCharacter 0)))
  (Variables|Default|SetPlayer _asbp_player))

(event EventInteract
  (switch int (Variables|Default|GetKeyIndex)
    (:1
      (Development|PrintString "Key1 Acquired")
      (Variables|/Game/BP_Player.BP_Player_C|SetAcquiredKey (Variables|Default|GetPlayer) "NewEnumerator1"))
    (:2
      (Development|PrintString "Key2 Acquired")
      (Variables|/Game/BP_Player.BP_Player_C|SetAcquiredKey (Variables|Default|GetPlayer) "NewEnumerator2"))
    (:3
      (Development|PrintString "Key3 Acquired")
      (Variables|/Game/BP_Player.BP_Player_C|SetAcquiredKey (Variables|Default|GetPlayer) "NewEnumerator3")))
  (Actor|DestroyActor))

(fn ConstructionScript)